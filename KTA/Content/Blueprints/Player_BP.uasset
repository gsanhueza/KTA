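; Player Blueprint that lets the player place traps and hazards in the world and forwards incoming damage to PlayerActions.
; Number keys 1-4 spawn a poison dart, bowling ball, spike blockade or land mine just ahead of the camera, using its rotation.
; K and J line trace from Arrow2 along the camera's forward vector and rotate a hit poison dart or spike blockade mesh in opposite directions.
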(event `self.ReceiveAnyDamage`
  (params (Damage :type "Float (single-precision)") (DamageType :type "DamageType Object Reference") (InstigatedBy :type "Controller Object Reference") (DamageCauser :type "Actor Object Reference"))
  (`PlayerActions.ReceiveDamage` (`self.PlayerActions`) Damage DamageType InstigatedBy DamageCauser))

(event `Key|One`
  (params (Key :type "Key Structure" :default "AnyKey"))
  (bind _transformcomponent (`PlayerCameraManager.TransformComponent` (`GameplayStatics.GetPlayerCameraManager` 0)))
  (:`Pressed`
    (`|SpawnActorFromClass` "/Game/KTA_Content/Turrets/PoisonDart_BP.PoisonDart_BP_C" (`KismetMathLibrary.MakeTransform` (+ (* (`SceneComponent.GetForwardVector` _transformcomponent) 200.0) (`SceneComponent.K2_GetComponentLocation` _transformcomponent)) (`SceneComponent.K2_GetComponentRotation` _transformcomponent)) "AdjustIfPossibleButAlwaysSpawn" "OverrideRootScale")))

(event `Key|Two`
  (params (Key :type "Key Structure" :default "AnyKey"))
  (bind _transformcomponent (`PlayerCameraManager.TransformComponent` (`GameplayStatics.GetPlayerCameraManager` 0)))
  (:`Pressed`
    (`|SpawnActorFromClass` "/Game/KTA_Content/Turrets/BowlingBall_BP.BowlingBall_BP_C" (`KismetMathLibrary.MakeTransform` (+ (* (`SceneComponent.GetForwardVector` _transformcomponent) 200.0) (`SceneComponent.K2_GetComponentLocation` _transformcomponent)) (`SceneComponent.K2_GetComponentRotation` _transformcomponent)) "AdjustIfPossibleButAlwaysSpawn" "OverrideRootScale")))

(event `Key|Three`
  (params (Key :type "Key Structure" :default "AnyKey"))
  (bind _transformcomponent (`PlayerCameraManager.TransformComponent` (`GameplayStatics.GetPlayerCameraManager` 0)))
  (:`Pressed`
    (`|SpawnActorFromClass` "/Game/KTA_Content/Turrets/SpikeBlockade_BP.SpikeBlockade_BP_C" (`KismetMathLibrary.MakeTransform` (+ (* (`SceneComponent.GetForwardVector` _transformcomponent) 200.0) (`SceneComponent.K2_GetComponentLocation` _transformcomponent)) (`SceneComponent.K2_GetComponentRotation` _transformcomponent)) "AdjustIfPossibleButAlwaysSpawn" "OverrideRootScale")))

(event `Key|Four`
  (params (Key :type "Key Structure" :default "AnyKey"))
  (bind _transformcomponent (`PlayerCameraManager.TransformComponent` (`GameplayStatics.GetPlayerCameraManager` 0)))
  (:`Pressed`
    (`|SpawnActorFromClass` "/Game/KTA_Content/Turrets/LandMine_BP.LandMine_BP_C" (`KismetMathLibrary.MakeTransform` (+ (* (`SceneComponent.GetForwardVector` _transformcomponent) 200.0) (`SceneComponent.K2_GetComponentLocation` _transformcomponent)) (`SceneComponent.K2_GetComponentRotation` _transformcomponent)) "Undefined" "OverrideRootScale")))

(event `Key|K`
  (params (Key :type "Key Structure" :default "AnyKey"))
  (bind _returnvalue (`SceneComponent.K2_GetComponentLocation` (`self.Arrow2`)))
  (:`Pressed`
    (bind _outhit (`KismetSystemLibrary.LineTraceSingle` _returnvalue (+ _returnvalue (* (`KismetMathLibrary.GetForwardVector` (`SceneComponent.K2_GetComponentRotation` (`PlayerCameraManager.TransformComponent` (`GameplayStatics.GetPlayerCameraManager` 0)))) 1500.0)) "TraceTypeQuery1"))
    (bind (_bblockinghit _binitialoverlap _time _location _impactpoint _normal _impactnormal _physmat _hitactor) (`GameplayStatics.BreakHitResult` _outhit))
    (cast `/Game/KTA_Content/Turrets/PoisonDart_BP` _hitactor
      (:`then`
        (bind _returnvalue_2 (`self.GetComponentByClass` _hitactor "/Script/Engine.StaticMeshComponent"))
        (`SceneComponent.K2_AddLocalRotation` _returnvalue_2 (struct :`Yaw` 10.0) false false))
      (:`CastFailed`
        (cast `/Game/KTA_Content/Turrets/SpikeBlockade_BP` _hitactor)
        (`SceneComponent.K2_AddLocalRotation` _returnvalue_2 (struct :`Yaw` 10.0) false false)))))

(event `Key|J`
  (params (Key :type "Key Structure" :default "AnyKey"))
  (bind _returnvalue (`SceneComponent.K2_GetComponentLocation` (`self.Arrow2`)))
  (:`Pressed`
    (bind _outhit (`KismetSystemLibrary.LineTraceSingle` _returnvalue (+ _returnvalue (* (`KismetMathLibrary.GetForwardVector` (`SceneComponent.K2_GetComponentRotation` (`PlayerCameraManager.TransformComponent` (`GameplayStatics.GetPlayerCameraManager` 0)))) 1500.0)) "TraceTypeQuery1"))
    (bind (_bblockinghit _binitialoverlap _time _location _impactpoint _normal _impactnormal _physmat _hitactor) (`GameplayStatics.BreakHitResult` _outhit))
    (cast `/Game/KTA_Content/Turrets/PoisonDart_BP` _hitactor
      (:`then`
        (bind _returnvalue_2 (`self.GetComponentByClass` _hitactor "/Script/Engine.StaticMeshComponent"))
        (`SceneComponent.K2_AddLocalRotation` _returnvalue_2 (struct :`Yaw` -10.0) false false))
      (:`CastFailed`
        (cast `/Game/KTA_Content/Turrets/SpikeBlockade_BP` _hitactor)
        (`SceneComponent.K2_AddLocalRotation` _returnvalue_2 (struct :`Yaw` -10.0) false false)))))

(fn `UserConstructionScript`)