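; CrystalCart_BP is the Blueprint for a crystal cart that displays its health on two health bar widgets.
; Every Tick it reads current and max health from CrystalCart and pushes their ratio to the Health_Bar widgets in the Health and Health2 components.
; The update is polled per frame rather than event-driven, and BeginPlay, overlap and construction logic are empty.
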(event `self.ReceiveTick`
  (params (DeltaSeconds :type "Float (single-precision)"))
  (bind _crystalcart (`self.CrystalCart`))
  (bind _returnvalue (`TurretComponent.getMaxHealth` _crystalcart))
  (bind _returnvalue_2 (`TurretComponent.getCurrentHealth` _crystalcart))
  (bind _ashealth_bar (cast `/Game/KTA_Content/Enemies/Widget+/Health_Bar` (`WidgetComponent.GetUserWidgetObject` (`self.Health`))))
  (bind _returnvalue_3 (/ _returnvalue_2 _returnvalue))
  (`/Game/KTA_Content/Enemies/Widget+/Health_Bar.SetPercent` _ashealth_bar _returnvalue_3)
  (bind _ashealth_bar_2 (cast `/Game/KTA_Content/Enemies/Widget+/Health_Bar` (`WidgetComponent.GetUserWidgetObject` (`self.Health2`))))
  (`/Game/KTA_Content/Enemies/Widget+/Health_Bar.SetPercent` _ashealth_bar_2 _returnvalue_3))

(event `self.ReceiveActorBeginOverlap`
  (params (OtherActor :type "Actor Object Reference")))

(fn `UserConstructionScript`)