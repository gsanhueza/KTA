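; Bear enemy Blueprint that walks constantly forward and reports its death state to its animation.
; Every Tick it overwrites the capsule's physics linear velocity along its forward vector, then adds a small downward velocity.
; It then reads the Dead result and copies it into the Muert variable of the Bear_Animation instance on its mesh.
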(event `self.ReceiveTick`
  (params (DeltaSeconds :type "Float (single-precision)"))
  (`PrimitiveComponent.SetPhysicsLinearVelocity` (`self.CapsuleComponent`) (* (`SceneComponent.GetForwardVector` (`self.CapsuleComponent`)) 100.0) false "None")
  (bind _returnvalue (`PrimitiveComponent.GetPhysicsLinearVelocity` (`self.CapsuleComponent`) "None"))
  (`PrimitiveComponent.SetPhysicsLinearVelocity` (`self.CapsuleComponent`) (+ (`KismetMathLibrary.MakeVector` 0.0 0.0 -20.0) _returnvalue) false "None")
  (bind _returnvalue_2 (`EnemyComponent.Dead` (`self.Bear`)))
  (bind _asbear_animation (cast `/Game/KTA_Content/Enemies/Bear/Bear_Animation` (`SkeletalMeshComponent.GetAnimInstance` (`self.Mesh`))))
  (set `/Game/KTA_Content/Enemies/Bear/Bear_Animation.muert` _returnvalue_2 _asbear_animation))

(fn `UserConstructionScript`)