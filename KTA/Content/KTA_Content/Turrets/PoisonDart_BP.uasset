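; PoisonDart turret Blueprint that damages Bear enemies entering its capsule.
; Capsule overlaps maintain a list of Characters in range, and a Tick accumulator deals fixed damage about once a second to the first entry if it is a Bear_BP.
; Tick also updates two health bar widgets from the PoisonDart health and destroys the actor when dead.
; A second five-second timer accumulates but triggers nothing.
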(event `self.ReceiveTick`
  (params (DeltaSeconds :type "Float (single-precision)"))
  (`self.Tick`)
  (bind _output_get (set `self.accumulator` (+ DeltaSeconds (`self.accumulator`))))
  (if (and (>= _output_get 1.0) (>= (`KismetArrayLibrary.Array_Length` (`self.Actores en Rango`)) 1))
    (set `self.accumulator` 0.0)
    (bind _asbear_bp (cast `/Game/KTA_Content/Enemies/Bear/Bear_BP` (`KismetArrayLibrary.Array_Get` (`self.Actores en Rango`))))
    (`EnemyComponent.ReceiveDamage` (`/Game/KTA_Content/Enemies/Bear/Bear_BP.Bear` _asbear_bp) 4.0 null null null)))

(event `self.Capsule.OnComponentBeginOverlap`
  (params (OverlappedComponent :type "PrimitiveComponent Object Reference") (OtherActor :type "Actor Object Reference") (OtherComp :type "PrimitiveComponent Object Reference") (OtherBodyIndex :type Integer) (bFromSweep :type Boolean) (SweepResult :type "HitResult Structure (by ref)"))
  (bind _ascharacter (cast `Character` OtherActor))
  (`KismetArrayLibrary.Array_Add` (`self.Actores en Rango`) _ascharacter))

(event `self.Capsule.OnComponentEndOverlap`
  (params (OverlappedComponent :type "PrimitiveComponent Object Reference") (OtherActor :type "Actor Object Reference") (OtherComp :type "PrimitiveComponent Object Reference") (OtherBodyIndex :type Integer))
  (bind _ascharacter (cast `Character` OtherActor))
  (`KismetArrayLibrary.Array_RemoveItem` (`self.Actores en Rango`) _ascharacter))

(event `Tick`
  (bind _poisondart (`self.PoisonDart`))
  (`self.Tick2`)
  (bind _returnvalue (`TurretComponent.getMaxHealth` _poisondart))
  (bind _returnvalue_2 (`TurretComponent.getCurrentHealth` _poisondart))
  (bind _ashealth_bar (cast `/Game/KTA_Content/Enemies/Widget+/Health_Bar` (`WidgetComponent.GetUserWidgetObject` (`self.HealthBar`))))
  (bind _returnvalue_3 (/ _returnvalue_2 _returnvalue))
  (`/Game/KTA_Content/Enemies/Widget+/Health_Bar.SetPercent` _ashealth_bar _returnvalue_3)
  (bind _ashealth_bar_2 (cast `/Game/KTA_Content/Enemies/Widget+/Health_Bar` (`WidgetComponent.GetUserWidgetObject` (`self.HealthBar2`))))
  (`/Game/KTA_Content/Enemies/Widget+/Health_Bar.SetPercent` _ashealth_bar_2 _returnvalue_3))

(event `Tick2`
  (`self.Tick3`)
  (bind _returnvalue (`TurretComponent.Dead` (`self.PoisonDart`)))
  (if _returnvalue
    (`self.K2_DestroyActor`)))

(event `Tick3`
  (bind _output_get (set `self.BAccumulator` (+ (stale `self.ReceiveTick` DeltaSeconds) (`self.BAccumulator`))))
  (if (>= _output_get 5.0)
    _))

(fn `UserConstructionScript`)