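; SpikeBlockade_BP is a spike blockade in the Turrets folder that displays its health on two health bar widgets.
; Every Tick it reads current and max health from SpikeBlockade, casts each widget component's user widget to Health_Bar and sets the percent to their ratio.
; BeginPlay, overlap and the construction script are empty, so this graph only drives the display.
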(event `self.ReceiveTick`
  (params (DeltaSeconds :type "Float (single-precision)"))
  (bind _spikeblockade (`self.SpikeBlockade`))
  (bind _returnvalue (`TurretComponent.getMaxHealth` _spikeblockade))
  (bind _returnvalue_2 (`TurretComponent.getCurrentHealth` _spikeblockade))
  (bind _ashealth_bar (cast `/Game/KTA_Content/Enemies/Widget+/Health_Bar` (`WidgetComponent.GetUserWidgetObject` (`self.HealthBar`))))
  (bind _returnvalue_3 (/ _returnvalue_2 _returnvalue))
  (`/Game/KTA_Content/Enemies/Widget+/Health_Bar.SetPercent` _ashealth_bar _returnvalue_3)
  (bind _ashealth_bar_2 (cast `/Game/KTA_Content/Enemies/Widget+/Health_Bar` (`WidgetComponent.GetUserWidgetObject` (`self.HealthBar2`))))
  (`/Game/KTA_Content/Enemies/Widget+/Health_Bar.SetPercent` _ashealth_bar_2 _returnvalue_3))

(event `self.ReceiveActorBeginOverlap`
  (params (OtherActor :type "Actor Object Reference")))

(fn `UserConstructionScript`)